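; BP_Boost is a pickup that sets CanUseBoost on a BP_Ball overlapping its mesh, then destroys itself.
; Each tick it yaws the actor at the Rotation rate and nudges the mesh along the actor's right vector.
; That position is projected by normalizing its offset from Earth and scaling to a fixed radius, applied around the world origin without re-adding Earth's location.
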(event `self.ReceiveTick`
  (params (DeltaSeconds :type "Float (single-precision)"))
  (`self.K2_AddActorWorldRotation` (`KismetMathLibrary.MakeRotator` 0.0 0.0 (* DeltaSeconds (`self.Rotation`))))
  (`SceneComponent.K2_SetWorldLocation` (`self.StaticMeshComponent`) (* (`KismetMathLibrary.Normal` (- (+ (`SceneComponent.K2_GetComponentLocation` (`self.StaticMeshComponent`)) (* (`self.GetActorRightVector`) (* DeltaSeconds 1000.0))) (`self.K2_GetActorLocation` (`self.Earth`)))) 5.0) false false))

(event `self.StaticMeshComponent.OnComponentBeginOverlap`
  (params (OverlappedComponent :type "PrimitiveComponent Object Reference") (OtherActor :type "Actor Object Reference") (OtherComp :type "PrimitiveComponent Object Reference") (OtherBodyIndex :type Integer) (bFromSweep :type Boolean) (SweepResult :type "HitResult Structure (by ref)"))
  (bind _asbp_ball (cast `/Game/Gameplay/Player/BP_Ball` OtherActor))
  (set `/Game/Gameplay/Player/BP_Ball.CanUseBoost` true _asbp_ball)
  (`self.K2_DestroyActor`))

(fn `UserConstructionScript`)