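; BP_FlyCamera is a shared camera that frames two players, P1 and P2, relative to an Earth actor.
; Each tick it finds the players' midpoint and places the camera a fixed distance beyond it along the direction away from Earth's origin.
; It then rotates the camera to look back at Earth's origin.
; Debug drawing and an alternative constraint-based offset remain in the graph but are unused.
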(event `self.ReceiveTick`
  (params (DeltaSeconds :type "Float (single-precision)"))
  (bind _returnvalue (`self.K2_GetActorLocation` (`self.P2`)))
  (bind _returnvalue_2 (`self.K2_GetActorLocation` (`self.Earth`)))
  (bind _returnvalue_3 (+ _returnvalue (/ (- (`self.K2_GetActorLocation` (`self.P1`)) _returnvalue) 2.0)))
  (`SceneComponent.K2_SetWorldLocation` (`self.CameraComponent`) (+ _returnvalue_3 (* (`KismetMathLibrary.Normal` (- _returnvalue_3 _returnvalue_2)) 700.0)) false false)
  (`SceneComponent.K2_SetWorldRotation` (`self.CameraComponent`) (`KismetMathLibrary.FindLookAtRotation` (`SceneComponent.K2_GetComponentLocation` (`self.CameraComponent`)) _returnvalue_2) false true))

(fn `UserConstructionScript`)