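; Controller that drives the flight of two physics-simulated player meshes toward shared targets.
; Prepare resets start positions, Shoot enables physics and targets an outer point, and Land freezes both.
; During Fly Phase, Tick applies impulses toward the target, scaled by a distance-based curve.
; A ball entering the inner sphere trigger retargets both to Earth; exiting swaps to the post-approach curve and locks further changes.
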(event `self.ReceiveBeginPlay`
  (`|ExecutionSequence`
    (:`then_0`
      (bind _output_get (set `self.Player1SM` (`self.GetComponentByClass` (`self.P1`) "/Script/Engine.StaticMeshComponent")))
      (set `self.P1_StartPos` (`SceneComponent.K2_GetComponentLocation` _output_get)))
    (:`then_1`
      (bind _output_get_2 (set `self.Player2SM` (`self.GetComponentByClass` (`self.P2`) "/Script/Engine.StaticMeshComponent")))
      (set `self.P2_StartPos` (`SceneComponent.K2_GetComponentLocation` _output_get_2)))))

(event `Land`
  (bind _player2sm (`self.Player2SM`))
  (`PrimitiveComponent.SetSimulatePhysics` _player2sm false)
  (`PrimitiveComponent.SetSimulatePhysics` (`self.Player1SM`) false)
  (`PrimitiveComponent.SetPhysicsLinearVelocity` (`self.Player1SM`) (0.0 0.0 0.0) false "None")
  (`PrimitiveComponent.SetPhysicsLinearVelocity` _player2sm (0.0 0.0 0.0) false "None")
  (`PrimitiveComponent.SetPhysicsAngularVelocityInDegrees` _player2sm (0.0 0.0 0.0) false "None")
  (`PrimitiveComponent.SetPhysicsAngularVelocityInDegrees` (`self.Player1SM`) (0.0 0.0 0.0) false "None"))

(event `Prepare`
  (`|ExecutionSequence`
    (:`then_0`
      (`SceneComponent.K2_SetWorldLocation` (`self.Player1SM`) (`self.P1_StartPos`) false true))
    (:`then_1`
      (`SceneComponent.K2_SetWorldLocation` (`self.Player2SM`) (`self.P2_StartPos`) false true))))

(event `Shoot`
  (bind _returnvalue (`self.GetComponentByClass` (`self.InnerSphereTrigger`) "/Script/Engine.SphereComponent"))
  (set `self.Target` (`self.OuterTargetPoint`))
  (`|ExecutionSequence`
    (:`then_0`
      (`PrimitiveComponent.SetSimulatePhysics` (`self.Player1SM`) true))
    (:`then_1`
      (`PrimitiveComponent.SetSimulatePhysics` (`self.Player2SM`) true))
    (:`then_2`
      (set `self.CurveToUse` "/Game/Gameplay/Player/BP_ApproachSpeed.BP_ApproachSpeed")
      (add `PrimitiveComponent.OnComponentBeginOverlap` _returnvalue (delegate `StartOverlap`))
      (add `PrimitiveComponent.OnComponentEndOverlap` _returnvalue (delegate `EndOverlap`)))))

(event `StartOverlap`
  (params (OverlappedComponent :type "PrimitiveComponent Object Reference") (OtherActor :type "Actor Object Reference") (OtherComp :type "PrimitiveComponent Object Reference") (OtherBodyIndex :type Integer) (bFromSweep :type Boolean) (SweepResult :type "HitResult Structure (by ref)"))
  (if (not (`self.LockChange`))
    (cast `/Game/Gameplay/Player/BP_Ball` OtherActor)
    (set `self.Target` (`self.Earth`))
    (remove `PrimitiveComponent.OnComponentBeginOverlap` (`self.GetComponentByClass` (`self.InnerSphereTrigger`) "/Script/Engine.SphereComponent") (delegate `StartOverlap`))))

(event `EndOverlap`
  (params (OverlappedComponent :type "PrimitiveComponent Object Reference") (OtherActor :type "Actor Object Reference") (OtherComp :type "PrimitiveComponent Object Reference") (OtherBodyIndex :type Integer))
  (if (not (`self.LockChange`))
    (cast `/Game/Gameplay/Player/BP_Ball` OtherActor)
    (set `self.CurveToUse` "/Game/Gameplay/Player/DistanceOverSpeedAfterApproach.DistanceOverSpeedAfterApproach")
    (set `self.LockChange` true)
    (remove `PrimitiveComponent.OnComponentEndOverlap` (`self.GetComponentByClass` (`self.InnerSphereTrigger`) "/Script/Engine.SphereComponent") (delegate `EndOverlap`))))

(event `self.ReceiveTick`
  (params (DeltaSeconds :type "Float (single-precision)"))
  (bind _target (`self.Target`))
  (bind _curvetouse (`self.CurveToUse`))
  (bind _returnvalue (- (`self.K2_GetActorLocation` _target) (`self.K2_GetActorLocation` (`self.P2`))))
  (bind _returnvalue_2 (- (`self.K2_GetActorLocation` _target) (`self.K2_GetActorLocation` (`self.P1`))))
  (switch `/Game/Blueprints/GameState` (`self.GameState`)
    (:`NewEnumerator2`
      (`PrimitiveComponent.AddImpulse` (`self.Player1SM`) (* (`KismetMathLibrary.Normal` _returnvalue_2) (`CurveFloat.GetFloatValue` _curvetouse (`KismetMathLibrary.VSize` _returnvalue_2))) "None" false)
      (`PrimitiveComponent.AddImpulse` (`self.Player2SM`) (* (`KismetMathLibrary.Normal` _returnvalue) (`CurveFloat.GetFloatValue` _curvetouse (`KismetMathLibrary.VSize` _returnvalue))) "None" false))))

(fn `UserConstructionScript`)