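; Camera and music manager that switches view and soundtrack across the game's main menu, shoot, fly and land phases.
; One MainCamera is the view target, and each Tick lerps its transform toward CurrentCamera by LerpSpeed, unscaled by delta time.
; SetCamera calls PlayMusic to swap tracks, then picks the camera and lerp speed.
; Fly follows without lag, while Land changes only the music.
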(event `PlayMusic`
  (params (Selection :type "/Game/Blueprints/GameState Enum" :default "NewEnumerator0"))
  (bind _audio_shoot (`self.Audio_Shoot`))
  (bind _audio_menu (`self.Audio_Menu`))
  (bind _audio_fly (`self.Audio_Fly`))
  (bind _audio_finale (`self.Audio_Finale`))
  (switch `/Game/Blueprints/GameState` Selection
    (:`NewEnumerator0`
      (`AudioComponent.Play` _audio_menu 0.0)
      (set `AudioComponent.VolumeMultiplier` 1.0 _audio_menu)
      (`AudioComponent.FadeOut` (`self.Audio_Finale`) 1.0 0.0))
    (:`NewEnumerator1`
      (`AudioComponent.FadeOut` _audio_menu 2.0 0.0)
      (`AudioComponent.FadeOut` _audio_finale 1.0 0.0)
      (`AudioComponent.Play` _audio_shoot 0.0))
    (:`NewEnumerator2`
      (`AudioComponent.Play` _audio_fly 0.0)
      (set `AudioComponent.VolumeMultiplier` 1.0 _audio_fly)
      (`AudioComponent.Stop` _audio_shoot))
    (:`NewEnumerator3`
      (`AudioComponent.Play` _audio_finale 0.0)
      (set `AudioComponent.VolumeMultiplier` 1.0 _audio_finale)
      (`AudioComponent.FadeOut` _audio_fly 1.0 0.0))))

(event `self.ReceiveBeginPlay`
  (`PlayerController.SetViewTargetWithBlend` (`GameplayStatics.GetPlayerController` 0) (`self.MainCamera`) 0.0 "VTBlend_Linear" 0.0 false))

(event `self.ReceiveTick`
  (params (DeltaSeconds :type "Float (single-precision)"))
  (bind _cameracomponent (`CameraActor.CameraComponent` (`self.MainCamera`)))
  (`SceneComponent.K2_SetWorldTransform` _cameracomponent (`KismetMathLibrary.TLerp` (`SceneComponent.K2_GetComponentToWorld` _cameracomponent) (`SceneComponent.K2_GetComponentToWorld` (`CameraActor.CameraComponent` (`self.CurrentCamera`))) (`self.LerpSpeed`)) false false))

(event `SetCamera`
  (params (Selection :type "/Game/Blueprints/GameState Enum" :default "NewEnumerator0"))
  (`self.PlayMusic` Selection)
  (switch `/Game/Blueprints/GameState` Selection
    (:`NewEnumerator0`
      (set `self.CurrentCamera` (`self.MenuCamera`))
      (set `self.LerpSpeed` 0.5 :!label _label))
    (:`NewEnumerator1`
      (set `self.CurrentCamera` (`self.ShootCamera`))
      (goto _label))
    (:`NewEnumerator2`
      (set `self.CurrentCamera` (`self.FlyCamera`))
      (set `self.LerpSpeed` 1.0))))

(fn `UserConstructionScript`)